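; Helper NPC Blueprint that shows its dialogue one line per Talk call in a WB_Dialogue widget.
; Talk advances TalkIndex through the Dialogue array and writes the line to the widget's NPCIntroduction text.
; When no valid widget exists, it creates one and adds it to the viewport without setting that line.
; Past the last line, it removes the widget from the viewport and resets the index to -1.
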(event EventTalk
  (Math|Integer|IncrementInt (Variables|Default|GettalkIndex)
    (:%20%20
      (if (< (Variables|Default|GettalkIndex) (Utilities|Array|Length (Variables|Default|Getdialogue)))
        (Variables|Default|GetUI
          (:then
            (Rendering|Components|TextRender|SetText (Variables|/Game/Dialogue/WB_Dialogue.WB_Dialogue_C|GetNPCIntroduction (Variables|Default|GetUI)) (Utilities|Text|ToText(String) (Utilities|Array|Get(acopy) (Variables|Default|Getdialogue) (Variables|Default|GettalkIndex)))))
          (:else
            (bind _returnvalue (UserInterface|CreateWidget "/Game/Dialogue/WB_Dialogue.WB_Dialogue_C" (Game|GetPlayerController 0)))
            (bind _output_get (Variables|Default|SetUI _returnvalue))
            (UserInterface|Viewport|AddtoViewport _output_get 0)))
        (else
          (Widget|RemovefromParent (Variables|Default|GetUI))
          (Variables|Default|SettalkIndex -1))))))

(fn ConstructionScript)